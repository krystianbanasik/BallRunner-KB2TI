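; Fall trigger actor that restarts the current level when any overlap with its FallTrigger component ends, with no check on the overlapping actor.
; After a 1.5-second delay it reopens the level by name, then starts a red camera fade-out, issued after the load call.
; BeginPlay fades in from the same red as a respawn effect.
; NewMacro_0 duplicates the restart sequence and is not called in the event graph.
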(event `self.fall trigger.OnComponentEndOverlap`
  (params (OverlappedComponent :type "PrimitiveComponent Object Reference") (OtherActor :type "Actor Object Reference") (OtherComp :type "PrimitiveComponent Object Reference") (OtherBodyIndex :type Integer))
  (bind _returnvalue (`GameplayStatics.GetCurrentLevelName` true))
  (`KismetSystemLibrary.Delay` 1.5)
  (`GameplayStatics.OpenLevel` (`KismetStringLibrary.Conv_StringToName` _returnvalue))
  (`PlayerCameraManager.StartCameraFade` (`PlayerController.PlayerCameraManager` (`GameplayStatics.GetPlayerController` 0)) 0.0 1.0 5.0 (struct :`R` 1.0 :`B` 0.040734 :`A` 1.0) false false))

(event `self.ReceiveBeginPlay`
  ;[1 1 1] fade po respie
  (`PlayerCameraManager.StartCameraFade` (`PlayerController.PlayerCameraManager` (`GameplayStatics.GetPlayerController` 0)) 1.0 0.0 5.0 (struct :`R` 1.0 :`B` 0.040734 :`A` 1.0) false false))

(fn `UserConstructionScript`)