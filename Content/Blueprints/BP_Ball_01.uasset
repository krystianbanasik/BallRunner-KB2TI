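; BP_Ball_01 is a player-controlled rolling ball that restarts the level when damaged.
; UpDown and LeftRight input axes apply torque to Sphere1 as an acceleration change.
; Space bar plays a timeline that offsets the sphere's Z from the actor location each update, apparently as a jump.
; The first damage event fades the camera to red, then reopens the current level after a delay.
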(event `InputAxis|UpDown`
  (params (AxisValue :type "Float (single-precision)"))
  (`PrimitiveComponent.AddTorqueInDegrees` (`self.Sphere1`) (`KismetMathLibrary.MakeVector` 0.0 (* AxisValue (`self.Multiply`))) "None" true))

(event `InputAxis|LeftRight`
  (params (AxisValue :type "Float (single-precision)"))
  (`PrimitiveComponent.AddTorqueInDegrees` (`self.Sphere1`) (`KismetMathLibrary.MakeVector` (* AxisValue (`self.Multiply`))) "None" true))

(event `Key|SpaceBar`
  (params (Key :type "Key Structure"))
  (bind (_returnvalue_x _returnvalue_y _returnvalue_z) (`KismetMathLibrary.BreakVector` (`self.K2_GetActorLocation`)))
  (:`Pressed`
    (bind (_direction _newtrack_0) (`Timeline|Timeline_0` :!via `PlayFromStart`)
      (:`Update`
        (`SceneComponent.K2_SetWorldLocation` (`self.Sphere1`) (`KismetMathLibrary.MakeVector` _returnvalue_x _returnvalue_y (+ (* (.z _newtrack_0) 15.0) _returnvalue_z)) false false)))))

(event `self.ReceiveAnyDamage`
  (params (Damage :type "Float (single-precision)") (DamageType :type "DamageType Object Reference") (InstigatedBy :type "Controller Object Reference") (DamageCauser :type "Actor Object Reference"))
  (`/Engine/EditorBlueprintResources/StandardMacros.DoOnce` false
    (:`Completed`
      (`PlayerCameraManager.StartCameraFade` (`PlayerController.PlayerCameraManager` (`GameplayStatics.GetPlayerController` 0)) 0.0 1.0 2.0 (struct :`R` 1.0 :`B` 0.040734 :`A` 1.0) false true)
      (bind _returnvalue (`GameplayStatics.GetCurrentLevelName` true))
      (`KismetSystemLibrary.Delay` 2.0)
      (`GameplayStatics.OpenLevel` (`KismetStringLibrary.Conv_StringToName` _returnvalue)))))

(fn `UserConstructionScript`)